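; BP_CameraActor is a trigger-driven cinematic camera that plays a sequence when a DefaultMovementCharacter enters its box.
; The overlap caches the character and its player controller, then starts SequencePlayer, whose play event blends the view to NewViewTarget.
; When the sequence stops, the view blends back to the character and both cached references are cleared.
; The reverse-play event is bound to an empty handler.
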(event `self.ReceiveBeginPlay`
  (bind _sequenceplayer (`self.SequencePlayer`))
  (add `MovieSceneSequencePlayer.OnPlay` _sequenceplayer (delegate `UpdateCamera`))
  (add `MovieSceneSequencePlayer.OnPlayReverse` _sequenceplayer (delegate `CameraTransformUpdate`))
  (add `MovieSceneSequencePlayer.OnStop` _sequenceplayer (delegate `Clear`)))

(event `UpdateCamera`
  (bind _as_player_controller (`self.As Player Controller`))
  (`/Engine/EditorBlueprintResources/StandardMacros.IsValid` _as_player_controller
    (:`Is Valid`
      (`PlayerController.SetViewTargetWithBlend` _as_player_controller (`self.New View Target`) 1.0 "VTBlend_Linear" 0.0 false))))

(event `CameraTransformUpdate`)

(event `Clear`
  (bind _as_player_controller (`self.As Player Controller`))
  (`/Engine/EditorBlueprintResources/StandardMacros.IsValid` _as_player_controller
    (:`Is Valid`
      (`PlayerController.SetViewTargetWithBlend` _as_player_controller (`self.As Default Movement Character`) 1.0 "VTBlend_Linear" 0.0 false)
      (set `self.As Default Movement Character` null)
      (set `self.As Player Controller` null))))

(event `self.Box.OnComponentBeginOverlap`
  (params (OverlappedComponent :type "PrimitiveComponent Object Reference") (OtherActor :type "Actor Object Reference") (OtherComp :type "PrimitiveComponent Object Reference") (OtherBodyIndex :type Integer) (bFromSweep :type Boolean) (SweepResult :type "HitResult Structure (by ref)"))
  (bind _asdefault_movement_character (cast `/Game/DefaultMovementCharacter` OtherActor))
  (set `self.As Default Movement Character` _asdefault_movement_character)
  (bind _asplayer_controller (cast `PlayerController` (`Pawn.GetController` _asdefault_movement_character)))
  (set `self.As Player Controller` _asplayer_controller)
  (`MovieSceneSequencePlayer.Play` (`self.SequencePlayer`)))

(fn `UserConstructionScript`)