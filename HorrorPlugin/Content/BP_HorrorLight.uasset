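; Horror light Blueprint that varies its brightness when its HorrorLightComponent is flagged as unstable.
; After the light state is set, it records the component's intensity multiplier and plays a timeline.
; Each timeline update overwrites the multiplier and refreshes the light.
; On finish, it sets a new timeline time through EffectTimeLineLoop and restores the recorded multiplier, without calling Play or UpdateLight again.
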(event `self.PostSetLightState`
  (bind _horrorlightcomponent (`self.HorrorLightComponent`))
  (if (`HorrorLightComponent.IsUnstable` (`self.HorrorLightComponent`))
    (set `self.RecordLightMultiflyIntencity` (`HorrorLightComponent.MultiflyIntensity` (`self.HorrorLightComponent`)))
    (bind (_direction _lightintencity) (`Timeline|LightUnstableTimeline` :!label _label)
      (:`Update`
        (set `HorrorLightComponent.MultiflyIntensity` _lightintencity _horrorlightcomponent)
        (`HorrorLightComponent.UpdateLight` _horrorlightcomponent))
      (:`Finished`
        (`self.EffectTimeLineLoop`)
        (set `HorrorLightComponent.MultiflyIntensity` (`self.RecordLightMultiflyIntencity`) (`self.HorrorLightComponent`))))))

(event `EffectTimeLineLoop`
  (goto _label :!via `SetNewTime`))

(fn `UserConstructionScript`)